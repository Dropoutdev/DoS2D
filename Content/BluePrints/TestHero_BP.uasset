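; Test hero character with side-scroller style movement along world X and a wall jump.
; Jump on the ground launches the character upward; while falling, it sphere-traces behind and ahead along the forward vector, using a span scaled from capsule radius.
; A hit launches it away from the impact along X at jump Z velocity, with debug prints and trace drawing left on.
; The construction script sets jump velocity and hold time.
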(event `InputAxis|moveRight`
  (params (AxisValue :type "Float (single-precision)"))
  ;[1 1 1] Movement
  (`self.AddMovementInput` (1.0 0.0 0.0) AxisValue))

(event `InputAction|Jump`
  (params (Key :type "Key Structure"))
  (bind _returnvalue_x (`KismetMathLibrary.BreakVector` (`self.K2_GetActorLocation`)))
  (:`Pressed`
    (if (`NavMovementComponent.IsFalling` (`self.CharacterMovement`))
      (bind (_start _end) (`self.Calc Start Pos`))
      (bind (_outhit _returnvalue) (`KismetSystemLibrary.SphereTraceSingle` :`Start` _start :`End` _end :`Radius` 50.0 :`TraceChannel` "TraceTypeQuery1" :`bTraceComplex` true :`DrawDebugType` "ForDuration"))
      (`KismetSystemLibrary.PrintString` (`KismetStringLibrary.Conv_BoolToString` _returnvalue))
      (if _returnvalue
        (bind _returnvalue_2 (`KismetMathLibrary.SignOfFloat` (- _returnvalue_x (.x (`.ImpactPoint` (`GameplayStatics.BreakHitResult` _outhit))))))
        (`KismetSystemLibrary.PrintString` (`KismetStringLibrary.Conv_DoubleToString` _returnvalue_2))
        (`self.LaunchCharacter` (`KismetMathLibrary.MakeVector` (* _returnvalue_2 1000.0) 0.0 (`CharacterMovementComponent.JumpZVelocity` (`self.CharacterMovement`))) true true))
      (else
        (`self.LaunchCharacter` (0.0 0.0 500.0))
        (set `self.JumpCount` (+ (`self.JumpCount`) 1)))))
  (:`Released`
    (`self.StopJumping`)))

(fn `Calc Start Pos`
  (returns (Start :type "Vector Structure") (end :type "Vector Structure"))
  (locals (`Scale Multiplier` :type "Float (double-precision)" :default 1.0))
  (bind _returnvalue (`self.GetActorForwardVector`))
  (bind _returnvalue_2 (* (`CapsuleComponent.GetScaledCapsuleRadius` (`self.CapsuleComponent`)) (`local.Scale Multiplier`)))
  (return (- (`self.K2_GetActorLocation`) (* _returnvalue _returnvalue_2)) (+ (* _returnvalue _returnvalue_2) (`self.K2_GetActorLocation`))))

(fn `UserConstructionScript`
  (set `CharacterMovementComponent.JumpZVelocity` 500.0 (`self.CharacterMovement`))
  (set `self.JumpMaxHoldTime` 0.3))