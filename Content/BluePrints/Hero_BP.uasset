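; Hero_BP is a 2D side-scrolling player character with sheep flipbooks, left/right movement and a double jump.
; The moveRight axis moves and turns the sprite, while A/D keys and jump timers set flags that AnimState turns into a flipbook each tick.
; A DoN node gates jump then launch, resetting on landing.
; A WallJump event line-traces for walls and launches away, but nothing here calls it.
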(event `UpdateAnim`
  ;[1 1 1] Anim Stuff To be changed
  (set `self.Is Moving?` (stale `Key|A` _output_get) :!label _label)
  (bind _flipbookoutput (`self.AnimState` (`self.Is Jump?`) (`self.Is Moving?`) (`self.Is Falling?`)))
  (`PaperFlipbookComponent.SetFlipbook` (`self.Sprite`) _flipbookoutput))

(event `self.ReceiveTick`
  (params (DeltaSeconds :type "Float (single-precision)"))
  ;[1 1 1] Anim Stuff To be changed
  (goto _label))

(event `Key|A`
  (params (Key :type "Key Structure"))
  ;[1 1 1] Anim Stuff To be changed
  (:`Pressed`
    (bind _output_get (set `self.Is Moving?` true :!label _label_2)))
  (:`Released`
    (set `self.Is Moving?` false :!label _label_3)))

(event `Key|D`
  (params (Key :type "Key Structure"))
  ;[1 1 1] Anim Stuff To be changed
  (:`Pressed`
    (goto _label_2))
  (:`Released`
    (goto _label_3)))

(event `InputAxis|moveRight`
  (params (AxisValue :type "Float (single-precision)"))
  (bind _sprite (`self.Sprite`))
  ;[1 1 1] Basic Movement Plus Anim
  (`self.UpdateAnim`)
  (if (> AxisValue 0.0)
    (`SceneComponent.K2_SetRelativeRotation` :`self` _sprite)
    (`self.AddMovementInput` (1.0 0.0 0.0) AxisValue :!label _label_4)
    (elif (< AxisValue 0.0)
      (`SceneComponent.K2_SetRelativeRotation` _sprite (struct :`Yaw` 180.0) false false)
      (goto _label_4))))

(event `InputAction|Jump`
  (params (Key :type "Key Structure"))
  ;[1 1 1] Anim Jump
  (:`Pressed`
    (bind _counter (`/Engine/EditorBlueprintResources/StandardMacros.Do N` 2 :!label _label_5)
      (:`Exit`
        (switch `int` _counter
          (:`1`
            (`self.Jump`)
            (set `self.Is Jump?` true)
            (`PaperFlipbookComponent.SetFlipbook` (`self.Sprite`) "/Game/Assests/SpriteSheets/SheepJump.SheepJump")
            (`KismetSystemLibrary.Delay` 0.3)
            (set `self.Is Jump?` false)
            (set `self.Is Falling?` true))
          (:`2`
            (set `self.Is Falling?` false)
            (set `self.Is Jump?` true)
            (`self.LaunchCharacter` (0.0 0.0 700.0))
            (`PaperFlipbookComponent.SetFlipbook` (`self.Sprite`) "/Game/Assests/SpriteSheets/SheepJump.SheepJump")
            (`KismetSystemLibrary.Delay` 0.3)
            (set `self.Is Jump?` false)
            (set `self.Is Falling?` true))))))
  (:`Released`
    (`self.StopJumping`)))

(event `self.OnLanded`
  (params (Hit :type "HitResult Structure (by ref)"))
  ;[1 1 1] Anim Jump
  (set `self.Is Jump?` false)
  (set `self.Is Falling?` false)
  (goto _label_5 :!via `Reset`))

(event `WallJump`
  (bind _returnvalue (`self.GetActorForwardVector`))
  (bind _returnvalue_x (`KismetMathLibrary.BreakVector` (`self.K2_GetActorLocation`)))
  (bind (_outhit _returnvalue_2) (`KismetSystemLibrary.LineTraceSingle` (- (`self.K2_GetActorLocation`) (* _returnvalue (+ (`CapsuleComponent.GetScaledCapsuleRadius` (`self.CapsuleComponent`)) 15.0))) (+ (`self.K2_GetActorLocation`) (* _returnvalue (+ (`CapsuleComponent.GetScaledCapsuleRadius` (`self.CapsuleComponent`)) 15.0))) "TraceTypeQuery1" true))
  (if _returnvalue_2
    (`self.LaunchCharacter` (`KismetMathLibrary.MakeVector` (* (`KismetMathLibrary.SignOfFloat` (- _returnvalue_x (.x (`.Location` (`GameplayStatics.BreakHitResult` _outhit))))) 450.0) 0.0 (`CharacterMovementComponent.JumpZVelocity` (`self.CharacterMovement`))) true true)))

(fn `AnimState`
  (params (`Is Jumping?` :type Boolean) (`IsMoving?` :type Boolean) (`Is Falling?` :type Boolean))
  (returns (FlipbookOutput :type "PaperFlipbook Object Reference"))
  (locals (animationState :type "/Game/BluePrints/Data/AnimState Enum") (`Is Falling Local` :type Boolean) (`Is Running Local` :type Boolean) (`Is Jumping Local` :type Boolean))
  (set `local.Is Jumping Local` `Is Jumping?`)
  (set `local.Is Running Local` `IsMoving?`)
  (set `local.Is Falling Local` `Is Falling?`)
  (if (`local.Is Falling Local`)
    (set `local.animationState` "NewEnumerator3")
    (elif (`local.Is Jumping Local`)
      (set `local.animationState` "NewEnumerator2")
      (elif (`local.Is Running Local`)
        (set `local.animationState` "NewEnumerator1")
        (else
          (set `local.animationState` "NewEnumerator0")))))
  (return (select `/Game/BluePrints/Data/AnimState` (`local.animationState`) :`NewEnumerator0` (`self.IdleFlipbook`) :`NewEnumerator1` (`self.RunFlipbook`) :`NewEnumerator2` (`self.JumpFlipbook`) :`NewEnumerator3` (`self.FallingFlipbook`))))

(fn `UserConstructionScript`)